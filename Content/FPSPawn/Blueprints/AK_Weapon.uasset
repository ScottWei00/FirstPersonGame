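; AK weapon for the first-person pawn, handling hitscan firing, effects and timed reloading.
; Fire spends ammo, plays sound and animation unless reloading, or dry-fires when empty.
; A randomly spread camera trace sets the aim point for a muzzle trace, which increments the pawn's Count on actors named "Cube".
; Shots spawn an impact decal and muzzle tracer; Reload plays a montage, then refills ammo after a delay.
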(event `self.Fire`
  (if (> (`self.Ammocount`) 0)
    (`self.AmmoCheck`) ; 进入开火处理函数
    (bind (_spawntransformloc _impact_point) (`self.LineTrace`)) ; 显示子弹发射轨迹
    (`self.SpawnDecalTracer` _spawntransformloc _impact_point _impact_point)
    (else
      (`GameplayStatics.PlaySoundAtLocation` "/Game/FPSPawn/SoundFX/DryFire.DryFire" (`SceneComponent.K2_GetComponentLocation` (`/Game/FPSPawn/Blueprints/FPSPawn_BP.FirstPersonCamera` (cast `/Game/FPSPawn/Blueprints/FPSPawn_BP` (`GameplayStatics.GetPlayerCharacter` 0) :!pure true))) (struct) 1.0 1.0 0.0 "/Game/FPSPawn/SoundFX/AK_Attenuation.AK_Attenuation" "/Game/FPSPawn/SoundFX/AK_Concurrency.AK_Concurrency" null) ; 播放无子弹声音
    )))

(event `self.Reload`
  (`SkeletalMeshComponent.PlayAnimation` (`self.PrimaryWeapon`) "/Game/FPSPawn/Animations/AK_Reload_anim_Montage.AK_Reload_anim_Montage" false) ; 加载枪动画
  (`KismetSystemLibrary.Delay` (`self.Reloadtime`))
  (set `self.Ammocount` (`self.MaxAmmo`)))

(fn `AmmoCheck`
  (bind _returnvalue (`KismetMathLibrary.RandomFloatInRange` 0.7 1.2))
  (`/Engine/EditorBlueprintResources/StandardMacros.DecrementInt` (`self.Ammocount`)
    (:`  `
      (if (not (`/Game/FPSPawn/Blueprints/FPSPawn_BP.IsReloading` (cast `/Game/FPSPawn/Blueprints/FPSPawn_BP` (`GameplayStatics.GetPlayerCharacter` 0) :!pure true)))
        (`GameplayStatics.PlaySoundAtLocation` "/Game/FPSPawn/SoundFX/Gunshot.Gunshot" (`SceneComponent.K2_GetComponentLocation` (`/Game/FPSPawn/Blueprints/FPSPawn_BP.FirstPersonCamera` (cast `/Game/FPSPawn/Blueprints/FPSPawn_BP` (`GameplayStatics.GetPlayerCharacter` 0) :!pure true))) (struct) (+ _returnvalue 2.5) _returnvalue 0.0 "/Game/FPSPawn/SoundFX/AK_Attenuation.AK_Attenuation" "/Game/FPSPawn/SoundFX/AK_Concurrency.AK_Concurrency" null) ; 播放有子弹声音
        (`SkeletalMeshComponent.PlayAnimation` (`self.PrimaryWeapon`) "/Game/FPSPawn/Animations/AK_Fire_anim.AK_Fire_anim" false) ; 播放枪动画
      ))))

(fn `LineTrace`
  (returns (SpawnTransformLoc :type "Vector Structure") (`Impact Point` :type "Vector Structure"))
  (bind _bulletspread (`self.BulletSpread`))
  (bind _returnvalue (`SceneComponent.K2_GetComponentLocation` (`self.Muzzle`)))
  (bind _returnvalue_2 (* -1 _bulletspread))
  (bind _firstpersoncamera (`/Game/FPSPawn/Blueprints/FPSPawn_BP.FirstPersonCamera` (cast `/Game/FPSPawn/Blueprints/FPSPawn_BP` (`GameplayStatics.GetPlayerCharacter` 0) :!pure true)))
  (bind _count (`/Game/FPSPawn/Blueprints/FPSPawn_BP.count` (cast `/Game/FPSPawn/Blueprints/FPSPawn_BP` (`GameplayStatics.GetPlayerCharacter` 0) :!pure true)))
  (bind _returnvalue_3 (`SceneComponent.K2_GetComponentLocation` _firstpersoncamera))
  (bind _outhit (`KismetSystemLibrary.LineTraceSingle` _returnvalue_3 (+ _returnvalue_3 (+ (* (`SceneComponent.GetForwardVector` _firstpersoncamera) 20000.0) (`KismetMathLibrary.MakeVector` (`KismetMathLibrary.RandomFloatInRange` _returnvalue_2 _bulletspread) (`KismetMathLibrary.RandomFloatInRange` _returnvalue_2 _bulletspread) (`KismetMathLibrary.RandomFloatInRange` _returnvalue_2 _bulletspread)))) "TraceTypeQuery1"))
  (bind (_bblockinghit _binitialoverlap _time _distance _location _impactpoint) (`GameplayStatics.BreakHitResult` _outhit))
  (bind (_outhit_2 _returnvalue_4) (`KismetSystemLibrary.LineTraceSingle` :`Start` _returnvalue :`End` _impactpoint :`TraceChannel` "TraceTypeQuery1" :`TraceColor` (struct :`R` 0.119833 :`G` 0.888668 :`B` 1.0 :`A` 1.0) :`TraceHitColor` (struct :`R` 0.054752 :`G` 0.046145 :`B` 1.0 :`A` 1.0) :`DrawTime` 1.0))
  (if _returnvalue_4
    (bind _returnvalue_5 (`KismetSystemLibrary.GetDisplayName` (`.HitActor` (`GameplayStatics.BreakHitResult` _outhit_2))))
    (`KismetSystemLibrary.PrintString` _returnvalue_5)
    (if (`KismetStringLibrary.EqualEqual_StrStr` _returnvalue_5 "Cube")
      (`/Engine/EditorBlueprintResources/StandardMacros.IncrementInt` _count
        (:`  `
          (`KismetSystemLibrary.PrintString` (`KismetStringLibrary.Conv_IntToString` _count))
          (return _returnvalue _impactpoint))))
    (else
      (`KismetSystemLibrary.PrintString` "Hello")
      (return _returnvalue _impactpoint))))

(fn `SpawnDecalTracer`
  (params (Location :type "Vector Structure") (SpawnTransformLo :type "Vector Structure") (ImpactPoint :type "Vector Structure"))
  (`|SpawnActorFromClass` "/Game/FPSPawn/Blueprints/BulletDecal_BP.BulletDecal_BP_C" (`KismetMathLibrary.MakeTransform` SpawnTransformLo (`KismetMathLibrary.Conv_VectorToRotator` ImpactPoint) (0.025 0.025 0.025)) "Undefined" "OverrideRootScale" null null) ; 子弹发射轨迹，打在物体上会留痕迹
  (if (>= (`KismetMathLibrary.RandomIntegerInRange` 1 10) 0)
    (`|SpawnActorFromClass` "/Game/FPSPawn/Blueprints/TraceRound_BP.TraceRound_BP_C" (`KismetMathLibrary.MakeTransform` Location (`SceneComponent.K2_GetComponentRotation` (`/Game/FPSPawn/Blueprints/FPSPawn_BP.FirstPersonCamera` (cast `/Game/FPSPawn/Blueprints/FPSPawn_BP` (`GameplayStatics.GetPlayerCharacter` 0) :!pure true))) (0.05 0.05 0.05)) "Undefined" "OverrideRootScale" null null) ; 子弹发出后的火花特效
  )
  (return))

(fn `UserConstructionScript`
  (`parent.UserConstructionScript`)
  (set `self.Ammocount` 30)
  (set `self.MaxAmmo` 30)
  (set `self.Reloadtime` 2.0)
  (set `self.BulletSpread` 500.0))